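; BP_FollowRotator is a component that smoothly turns a given scene component to face a target actor over a set rotation time.
; An init function stores both references, and StartRotating guards against zero duration, captures start and look-at rotations once, then activates it.
; Tick lerps world rotation by elapsed-time progress and deactivates the component on completion, so target movement during a turn is not tracked.
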(event `self.ReceiveTick`
  (params (DeltaSeconds :type "Float (single-precision)"))
  (bind _currentprogress (`self.CalculateProgress`))
  (`|ExecutionSequence`
    (:`then_0`
      (set `self.PassedTime` (`KismetMathLibrary.FClamp` (+ DeltaSeconds (`self.PassedTime`)) 0.0 (`self.RotationTIme`))))
    (:`then_1`
      (`|ExecutionSequence`
        (:`then_0`
          (`SceneComponent.K2_SetWorldRotation` (`self.RotatingComponent`) (`KismetMathLibrary.RLerp` (`self.StartRotation`) (`self.FinalRotation`) _currentprogress) false false))
        (:`then_1`
          (if (`KismetMathLibrary.NearlyEqual_FloatFloat` _currentprogress 1.0)
            (`self.OnFinishRotating`)))))))

(event `OnFinishRotating`
  (`self.SetActive` false))

(fn `CalculateProgress`
  (returns (CurrentProgress :type "Float (double-precision)"))
  (return (/ (`self.PassedTime`) (`self.RotationTIme`))))

(fn `CaptureRotationData`
  (bind _rotatingcomponent (`self.RotatingComponent`))
  (`|ExecutionSequence`
    (:`then_0`
      (set `self.StartRotation` (`SceneComponent.K2_GetComponentRotation` _rotatingcomponent)))
    (:`then_1`
      (set `self.FinalRotation` (`KismetMathLibrary.FindLookAtRotation` (`SceneComponent.K2_GetComponentLocation` _rotatingcomponent) (`Actor.K2_GetActorLocation` (`self.TargetActor`)))))))

(fn `InitializeFallowingRotationFor`
  (params (RotatingComponent :type "SceneComponent Object Reference") (TargetActor :type "Actor Object Reference"))
  (`|ExecutionSequence`
    (:`then_0`
      (set `self.RotatingComponent` RotatingComponent))
    (:`then_1`
      (set `self.TargetActor` TargetActor))))

(fn `StartRotating`
  (`|ExecutionSequence`
    (:`then_0`
      (if (`KismetMathLibrary.NearlyEqual_FloatFloat` (`self.RotationTIme`))
        (set `self.RotationTIme` 0.01)))
    (:`then_1`
      (set `self.PassedTime` 0.0)
      (`self.CaptureRotationData`)
      (`self.SetActive` true))))
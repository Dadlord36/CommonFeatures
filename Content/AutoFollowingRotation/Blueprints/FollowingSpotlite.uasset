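; FollowingSpotlite is an actor whose SpotLight rotates to follow a BP_MovableTarget found in the world.
; On BeginPlay it looks up the target, prints a message if none exists, and initializes its BPFollowRotator with the light and target.
; Rotation starts immediately.
; Tick compares the target's location with the cached previous one and calls StartRotating again whenever it moves, leaving the rotation itself to BPFollowRotator.
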(event `self.ReceiveBeginPlay`
  (bind _bp_followrotator (`self.BP_FollowRotator`))
  (`|ExecutionSequence`
    (:`then_0`
      ;[1 1 1] Find target actor in the world
      (bind _returnvalue (`GameplayStatics.GetActorOfClass` "/CommonFeatures/AutoFollowingRotation/Blueprints/BP_MovableTarget.BP_MovableTarget_C"))
      (bind _output_get (set `self.TargetActor` _returnvalue))
      (`/Engine/EditorBlueprintResources/StandardMacros.IsValid` _output_get
        (:`Is Not Valid`
          (`KismetSystemLibrary.PrintString` "So actor was not found and so the system won't work."))))
    (:`then_1`
      ;[1 1 1] Initialize rotator and start following target
      (`/CommonFeatures/AutoFollowingRotation/Blueprints/BP_FollowRotator.InitializeFallowingRotationFor` _bp_followrotator (`self.SpotLight`) (`self.TargetActor`))
      (`/CommonFeatures/AutoFollowingRotation/Blueprints/BP_FollowRotator.StartRotating` _bp_followrotator))))

(event `self.ReceiveTick`
  (params (DeltaSeconds :type "Float (single-precision)"))
  (if (`self.IsActorPositionChanged`)
    (`self.OnTargetChangePosition`)))

(event `OnTargetChangePosition`
  (`/CommonFeatures/AutoFollowingRotation/Blueprints/BP_FollowRotator.StartRotating` (`self.BP_FollowRotator`)))

(fn `IsActorPositionChanged`
  (returns (ReturnValue :type Boolean))
  (locals (Result :type Boolean))
  (bind _targetactor (`self.TargetActor`))
  (bind _returnvalue (`self.K2_GetActorLocation` _targetactor))
  (`/Engine/EditorBlueprintResources/StandardMacros.IsValid` _targetactor
    (:`Is Valid`
      (set `local.Result` (!= _returnvalue (`self.PreviousPosition`) :`ErrorTolerance` 0.001))
      (set `self.PreviousPosition` _returnvalue)
      (return (`local.Result`)))))

(fn `UserConstructionScript`)